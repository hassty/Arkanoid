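; Base game state that tracks the round's state and elapsed time.
; Tick, noted as running once per second, advances the round time while in progress and ends the game when the game mode's optional time limit is reached.
; The RoundState RepNotify prints state changes, switches the first player to game-only input on start, and fires game started and ended calls.
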(event `self.ReceiveTick`
  (params (DeltaSeconds :type "Float (single-precision)"))
  ;[1 1 1] Round Timer
  (switch `/Game/Data/Enums/E_RoundState` (`self.RoundState`)
    (:`NewEnumerator1`
      (`self.RoundTimeTick`))))

(fn `OnRep_RoundState`
  (bind _gamemode (`/Game/Blueprints/Libs/Functions/BP_Functions_GlobalGetters.GetGameMode`))
  (bind _returnvalue (`GameplayStatics.GetPlayerController` 0))
  (switch `/Game/Data/Enums/E_RoundState` (`self.RoundState`)
    (:`NewEnumerator1`
      (set `/Game/Blueprints/Game/BP_BaseGamemode.GameStyle` (`/Game/Blueprints/Game/BP_BaseGamemode.GameStyle` _gamemode) _gamemode)
      (`WidgetBlueprintLibrary.SetInputMode_GameOnly` _returnvalue)
      (set `PlayerController.bShowMouseCursor` false _returnvalue)
      (`KismetSystemLibrary.PrintString` "Game started" true true (struct :`R` 0.2 :`G` 1.0 :`A` 1.0) 2.0)
      (`self.GameStarted`))
    (:`NewEnumerator3`
      (`KismetSystemLibrary.PrintString` "Game paused" true true (struct :`R` 0.2 :`G` 1.0 :`A` 1.0)))
    (:`NewEnumerator2`
      (`KismetSystemLibrary.PrintString` "Game ended" true true (struct :`R` 0.2 :`G` 1.0 :`A` 1.0))
      (`self.GameEnded`))))

(fn `RoundTimeTick`
  (bind _gamemode (`/Game/Blueprints/Libs/Functions/BP_Functions_GlobalGetters.GetGameMode`))
  (set `self.RoundTime` (+ (`self.RoundTime`) (`KismetMathLibrary.MakeTimespan` 0 0 0 1)))
  (if (`/Game/Blueprints/Game/BP_BaseGamemode.LimitByTime` _gamemode)
    (if (>= (`self.RoundTime`) (`/Game/Blueprints/Game/BP_BaseGamemode.TimeLimit` _gamemode))
      (set `self.RoundState` "NewEnumerator2"))))

(fn `UserConstructionScript`)