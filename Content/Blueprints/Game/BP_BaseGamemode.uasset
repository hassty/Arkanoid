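; Base game mode that sets the game state's round state on BeginPlay and handles scoring for destroyed obstacles.
; ObstacleDestroyed adds the passed score to the first player controller's player state, and the GameStyle RepNotify calls GameStyleChanged with the new style.
; Score and time limit checks are empty stubs, with the ScoreLimitReached call left in unconnected nodes.
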(event `self.ReceiveBeginPlay`
  (set `/Game/Blueprints/Game/BP_BaseGameState.RoundState` "NewEnumerator1" (`/Game/Blueprints/Libs/Functions/BP_Functions_GlobalGetters.GetGameState`)))

(fn `CheckScoreLimit`)

(fn `CheckTimeLimit`)

(fn `ObstacleDestroyed`
  (params (Score :type Integer))
  (`/Game/Blueprints/Player/BP_PlayerState.AddScore` (`/Game/Blueprints/Libs/Functions/BP_Functions_GlobalGetters.GetPlayerStateByController` (`GameplayStatics.GetPlayerController` 0)) Score))

(fn `OnRep_GameStyle`
  (`self.GameStyleChanged` (`self.GameStyle`)))

(fn `UserConstructionScript`)