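; Base HUD that shows and hides the main menu, in-game HUD, settings and levels widgets.
; Each Toggle function creates its widget on first show and caches it; menu screens set UI-only input, and settings and levels also change the game state's RoundState.
; OnGameStarted swaps the main menu for the HUD, but its binding and the initial menu display are disconnected, leaving BeginPlay empty.
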(event `self.ReceiveBeginPlay`)

(event `OnGameStarted`
  (`self.ToggleMenu` false)
  (`self.ToggleHUD` true))

(fn `ToggleHUD`
  (params (Show :type Boolean))
  (if Show
    (`self.W_HUD`
      (:`then`
        _)
      (:`else`
        (bind _returnvalue (`|CreateWidget` (`self.W_HUDClass`) (`self.GetOwningPlayerController`)))
        (bind _output_get (set `self.W_HUD` _returnvalue))))
    (`UserWidget.AddToViewport` _output_get 0)
    (else
      (bind _w_hud (`self.W_HUD`)
        (:`then`
          (`Widget.RemoveFromParent` _w_hud))
        (:`else`)))))

(fn `ToggleLevels`
  (params (Show :type Boolean))
  (bind _returnvalue (`self.GetOwningPlayerController`))
  (if Show
    (`self.W_Levels`
      (:`then`
        _)
      (:`else`
        (bind _returnvalue_2 (`|CreateWidget` (`self.W_LevelsClass`) _returnvalue))
        (bind _output_get (set `self.W_Levels` _returnvalue_2))))
    (`UserWidget.AddToViewport` _output_get 0)
    (`WidgetBlueprintLibrary.SetInputMode_UIOnlyEx` _returnvalue _output_get)
    (set `/Game/Blueprints/Game/BP_BaseGameState.RoundState` "NewEnumerator3" (`/Game/Blueprints/Libs/Functions/BP_Functions_GlobalGetters.GetGameState`))
    (else
      (bind _w_levels (`self.W_Levels`)
        (:`then`
          (`Widget.RemoveFromParent` _w_levels))
        (:`else`)))))

(fn `ToggleMenu`
  (params (Show :type Boolean))
  (bind _returnvalue (`self.GetOwningPlayerController`))
  (if Show
    (`self.W_MainMenu`
      (:`then`
        _)
      (:`else`
        (bind _returnvalue_2 (`|CreateWidget` (`self.W_MainMenuClass`) _returnvalue))
        (bind _output_get (set `self.W_MainMenu` _returnvalue_2))))
    (`UserWidget.AddToViewport` _output_get 0)
    (`WidgetBlueprintLibrary.SetInputMode_UIOnlyEx` _returnvalue (`/Game/UI/HUD/MainMenu/W_MainMenuTab.B_Start` (`/Game/UI/HUD/MainMenu/W_HUD_MainMenu.W_MainMenuTab` _output_get)))
    (set `PlayerController.bShowMouseCursor` true _returnvalue)
    (else
      (bind _w_mainmenu (`self.W_MainMenu`)
        (:`then`
          (`Widget.RemoveFromParent` _w_mainmenu))
        (:`else`)))))

(fn `ToggleSettings`
  (params (Show :type Boolean))
  (bind _returnvalue (`self.GetOwningPlayerController`))
  (if Show
    (`self.W_Settings`
      (:`then`
        _)
      (:`else`
        (bind _returnvalue_2 (`|CreateWidget` (`self.W_SettingsClass`) _returnvalue))
        (bind _output_get (set `self.W_Settings` _returnvalue_2))))
    (`UserWidget.AddToViewport` _output_get 0)
    (`WidgetBlueprintLibrary.SetInputMode_UIOnlyEx` _returnvalue _output_get)
    (set `/Game/Blueprints/Game/BP_BaseGameState.RoundState` "NewEnumerator3" (`/Game/Blueprints/Libs/Functions/BP_Functions_GlobalGetters.GetGameState`))
    (else
      (bind _w_settings (`self.W_Settings`)
        (:`then`
          (`Widget.RemoveFromParent` _w_settings))
        (:`else`)))))

(fn `UserConstructionScript`)