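; BP_ObstacleManager fills the level with a grid of obstacle actors when the game starts.
; It binds to the GameState's GameStarted event on BeginPlay, and a BuildLevel event runs the same spawn logic.
; Nested loops spawn ObstacleClass at a fixed height, spaced by mesh size plus an offset.
; Positions are absolute world coordinates, independent of the manager's own location.
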(event `self.ReceiveBeginPlay`
  (add `/Game/Blueprints/Game/BP_BaseGameState.GameStarted` (`/Game/Blueprints/Libs/Functions/BP_Functions_GlobalGetters.GetGameState`) (delegate `OnGameStarted`)))

(event `OnGameStarted`
  (bind _meshoffset (`self.MeshOffset`))
  (for _index (range 1 (+ (`self.СounterY`) 1)) :!label _label
    (for _index_2 (range 1 (+ (`self.CounterX`) 1))
      (`|SpawnActorFromClass` (`self.ObstacleClass`) (`KismetMathLibrary.MakeTransform` (`KismetMathLibrary.MakeVector` (* _index (+ (`self.MeshWidth`) _meshoffset)) (* _index_2 (+ (`self.MeshLength`) _meshoffset)) 100.0)) "AdjustIfPossibleButAlwaysSpawn" "OverrideRootScale" null null))))

(event `BuildLevel`
  (goto _label))

(fn `UserConstructionScript`)