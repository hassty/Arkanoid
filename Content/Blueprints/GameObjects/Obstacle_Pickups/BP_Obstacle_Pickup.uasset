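; Obstacle pickup that activates for a set time when anything overlaps its sphere, with a construction script tinting its mesh by a Color variable.
; Overlap sets the Using RepNotify, whose handler hides the actor, disables collision, calls UsePickup and starts a UsingTime timer.
; When the timer clears Using, the same handler calls StopUsePickup and destroys the actor.
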(event `self.Sphere.OnComponentBeginOverlap`
  (params (OverlappedComponent :type "PrimitiveComponent Object Reference") (OtherActor :type "Actor Object Reference") (OtherComp :type "PrimitiveComponent Object Reference") (OtherBodyIndex :type Integer) (bFromSweep :type Boolean) (SweepResult :type "HitResult Structure (by ref)"))
  (`self.Use`))

(fn `OnRep_Using`
  (if (`self.Using`)
    (`self.SetActorHiddenInGame` true)
    (`self.SetActorEnableCollision` false)
    (bind _returnvalue (`KismetSystemLibrary.K2_SetTimer` null "StopUsing" (`self.UsingTime`)))
    (set `self.UsingTimer` _returnvalue)
    (`self.UsePickup`)
    (else
      (`KismetSystemLibrary.K2_ClearAndInvalidateTimerHandle` (`self.UsingTimer`))
      (`self.StopUsePickup`)
      (`self.K2_DestroyActor`))))

(fn `StartUsing`
  (bind _returnvalue (`KismetSystemLibrary.K2_SetTimer` null "StopUsing" (`self.UsingTime`)))
  (set `self.UsingTimer` _returnvalue))

(fn `StopUsing`
  (set `self.Using` false))

(fn `Use`
  (if (not (`self.Using`))
    (set `self.Using` true)))

(fn `UserConstructionScript`
  (bind _returnvalue (`PrimitiveComponent.CreateDynamicMaterialInstance` (`self.Sphere1`) 0 "/Game/Assets/Materials/M_BaseMat.M_BaseMat"))
  (`MaterialInstanceDynamic.SetVectorParameterValue` _returnvalue "Color" (`self.Color`)))