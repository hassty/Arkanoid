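; Timed or toggled obstacle pickup that widens the player's platform along its Y axis while in use.
; On BeginPlay it binds to the UsePickup and StopUsePickup dispatchers.
; On use it sets the controlled BP_PlayerPawn's Platform to a fixed world Y scale, keeping X and Z.
; On stop it restores the platform from the pawn's stored Scale variable.
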(event `self.ReceiveBeginPlay`
  (add `self.UsePickup` (delegate `OnUsePickup`))
  (add `self.StopUsePickup` (delegate `OnStopUsePickup`)))

(event `OnUsePickup`
  (bind _platform (`/Game/Blueprints/Player/BP_PlayerPawn.Platform` (cast `/Game/Blueprints/Player/BP_PlayerPawn` (`Controller.K2_GetPawn` (`GameplayStatics.GetPlayerController` 0)) :!pure true)))
  (bind (_returnvalue_x _returnvalue_y _returnvalue_z) (`KismetMathLibrary.BreakVector` (`SceneComponent.K2_GetComponentScale` _platform)))
  (`SceneComponent.SetWorldScale3D` _platform (`KismetMathLibrary.MakeVector` _returnvalue_x 3.5 _returnvalue_z)))

(event `OnStopUsePickup`
  (bind _asbp_player_pawn (cast `/Game/Blueprints/Player/BP_PlayerPawn` (`Controller.K2_GetPawn` (`GameplayStatics.GetPlayerController` 0)) :!pure true))
  (`SceneComponent.SetWorldScale3D` (`/Game/Blueprints/Player/BP_PlayerPawn.Platform` _asbp_player_pawn) (`/Game/Blueprints/Player/BP_PlayerPawn.Scale` _asbp_player_pawn)))

(fn `UserConstructionScript`
  (`parent.UserConstructionScript`))