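; A speed pickup obstacle that temporarily changes the player pawn's movement speed.
; On BeginPlay it binds handlers to the pickup's use and stop-use dispatchers.
; Use sets the controlled BP_PlayerPawn's MovementSpeed to PickupMovementSpeed, and stop-use restores it to the pawn's MaxMovementSpeed.
; The construction script only calls its parent.
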(event `self.ReceiveBeginPlay`
  (add `self.UsePickup` (delegate `OnUsePickup`))
  (add `self.StopUsePickup` (delegate `OnStopUsePickup`)))

(event `OnUsePickup`
  (set `/Game/Blueprints/Player/BP_PlayerPawn.MovementSpeed` (`self.PickupMovementSpeed`) (cast `/Game/Blueprints/Player/BP_PlayerPawn` (`Controller.K2_GetPawn` (`GameplayStatics.GetPlayerController` 0)) :!pure true)))

(event `OnStopUsePickup`
  (bind _asbp_player_pawn (cast `/Game/Blueprints/Player/BP_PlayerPawn` (`Controller.K2_GetPawn` (`GameplayStatics.GetPlayerController` 0)) :!pure true))
  (set `/Game/Blueprints/Player/BP_PlayerPawn.MovementSpeed` (`/Game/Blueprints/Player/BP_PlayerPawn.MaxMovementSpeed` _asbp_player_pawn) _asbp_player_pawn))

(fn `UserConstructionScript`
  (`parent.UserConstructionScript`))