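; BP_Obstacle is a destructible obstacle that takes hits, awards score and drops a pickup.
; The construction script resets HP to its maximum and tints the cube through a dynamic material instance.
; Each cube hit runs HPCheck, which decrements HP and, at zero, reports the score to the game mode and destroys the actor.
; Destruction spawns the pickup class in place; a leftover grid-spawning loop is disconnected and never runs.
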(event `self.Cube.OnComponentHit`
  (params (HitComponent :type "PrimitiveComponent Object Reference") (OtherActor :type "Actor Object Reference") (OtherComp :type "PrimitiveComponent Object Reference") (NormalImpulse :type "Vector Structure") (Hit :type "HitResult Structure (by ref)"))
  (`self.HPCheck`))

(event `self.ReceiveDestroyed`
  (`|SpawnActorFromClass` (`self.PickupClass`) (`KismetMathLibrary.MakeTransform` (`self.K2_GetActorLocation`)) "AlwaysSpawn" "OverrideRootScale" null null))

(fn `HPCheck`
  (`/Engine/EditorBlueprintResources/StandardMacros.DecrementInt` (`self.HP`)
    (:`  `
      (if (<= (`self.HP`) 0)
        (`/Game/Blueprints/Game/BP_BaseGamemode.ObstacleDestroyed` (`/Game/Blueprints/Libs/Functions/BP_Functions_GlobalGetters.GetGameMode`) (`self.Score`))
        (`self.K2_DestroyActor`)))))

(fn `UserConstructionScript`
  (set `self.HP` (`self.MaxHP`))
  (bind _returnvalue (`PrimitiveComponent.CreateDynamicMaterialInstance` (`self.Cube`) 0 "/Game/Assets/Materials/M_BaseMat.M_BaseMat"))
  (`MaterialInstanceDynamic.SetVectorParameterValue` _returnvalue "Color" (`self.Color`)))