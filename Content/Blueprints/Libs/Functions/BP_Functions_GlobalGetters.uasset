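; BP_Functions_GlobalGetters is a function library of shortcuts that return core gameplay framework objects already cast to the project's own classes.
; It fetches the game mode as BP_BaseGameMode, the game state as BP_BaseGameState and a given controller's player state as BP_PlayerState.
; GetGameSettings returns the game instance cast to GI_Settings, so the game instance serves as the settings object.
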(fn `GetGameMode`
  (returns (GameMode :type "/Game/Blueprints/Game/BP_BaseGamemode Object Reference"))
  (return (cast `/Game/Blueprints/Game/BP_BaseGamemode` (`GameplayStatics.GetGameMode` null) :!pure true)))

(fn `GetGameSettings`
  (returns (Settings :type "/Game/Blueprints/Game/GI_Settings Object Reference"))
  (return (cast `/Game/Blueprints/Game/GI_Settings` (`GameplayStatics.GetGameInstance` null) :!pure true)))

(fn `GetGameState`
  (returns (GameState :type "/Game/Blueprints/Game/BP_BaseGameState Object Reference"))
  (return (cast `/Game/Blueprints/Game/BP_BaseGameState` (`GameplayStatics.GetGameState` null) :!pure true)))

(fn `GetPlayerStateByController`
  (params (Controller :type "Controller Object Reference"))
  (returns (PlayerState :type "/Game/Blueprints/Player/BP_PlayerState Object Reference"))
  (return (cast `/Game/Blueprints/Player/BP_PlayerState` (`Controller.PlayerState` Controller) :!pure true)))