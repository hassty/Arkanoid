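; Player state Blueprint that tracks score and hit points for the player pawn, which it caches on BeginPlay.
; HP changes one point at a time: gains cap at the maximum, a non-lethal loss makes the pawn spawn a projectile, and zero destroys it.
; A RepNotify on PlayerHP sets an HP state enum at full, half and quarter-or-below thresholds, then refreshes the pawn's HP bar widget.
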(event `self.ReceiveBeginPlay`
  (set `self.PlayerPawn` (cast `/Game/Blueprints/Player/BP_PlayerPawn` (`Controller.K2_GetPawn` (`GameplayStatics.GetPlayerController` 0)) :!pure true))
  (set `self.PlayerHP` (`self.MaxPlayerHP`)))

(fn `AddScore`
  (params (Score :type Integer))
  (set `self.PlayerScore` (+ (`self.PlayerScore`) Score)))

(fn `OnRep_PlayerHP`
  (`self.SetPlayerHPState`)
  (`/Game/UI/HUD/Health/W_HP_Bar.UpdateHPBar` (cast `/Game/UI/HUD/Health/W_HP_Bar` (`WidgetComponent.GetUserWidgetObject` (`/Game/Blueprints/Player/BP_PlayerPawn.W_HP` (`self.PlayerPawn`))) :!pure true)))

(fn `SetPlayerHP`
  (params (Add :type Boolean))
  (bind _playerhp (`self.PlayerHP`))
  (bind _playerpawn (`self.PlayerPawn`))
  (if Add
    (set `self.PlayerHP` (`KismetMathLibrary.Min` (+ _playerhp 1) (`self.MaxPlayerHP`)))
    (else
      (set `self.PlayerHP` (- _playerhp 1))
      (if (<= (`self.PlayerHP`) 0)
        (`self.K2_DestroyActor` _playerpawn)
        (else
          (`/Game/Blueprints/Player/BP_PlayerPawn.SpawnProjectile` _playerpawn true))))))

(fn `SetPlayerHPState`
  (if (== (`self.PlayerHP`) (`self.MaxPlayerHP`))
    (set `self.PlayerStateHP` "NewEnumerator2")
    (elif (== (`self.PlayerHP`) (`KismetMathLibrary.Round` (* (`self.MaxPlayerHP`) 0.5)))
      (set `self.PlayerStateHP` "NewEnumerator1")
      (elif (<= (`self.PlayerHP`) (`KismetMathLibrary.Round` (* (`self.MaxPlayerHP`) 0.25)))
        (set `self.PlayerStateHP` "NewEnumerator0")))))

(fn `UserConstructionScript`)